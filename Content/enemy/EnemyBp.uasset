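; Base enemy Blueprint that holds health, takes damage and credits kills to the attacking player.
; TakeDamge runs only with authority, subtracting health, calling empty child-override hooks for hit and death, and adding a destroy count to the PlayerState found by player index.
; ProcessBound, also authority-only, destroys the enemy once its X falls below the GameState's start X plus move length.
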(event EventBeginPlay)

(event Collision|EventActorBeginOverlap
  (params (OtherActor :type Actor%20Object%20Reference)))

(event EventTick
  (params (DeltaSeconds :type Float%20%28single-precision%29)))

(fn ConstructionScript)

(fn BeginDestroy)

(fn TakeDamge
  (params (damge :type Integer) (playerindex :type Integer))
  (if (Ability|HasAuthority)
    (bind _output_get (Variables|Default|Set_heath (- (Variables|Default|Get_heath) damge)))
    (CallFunction|TakeDamgebyChild playerindex)
    (if (<= _output_get 0)
      (CallFunction|ProcessDestroybyChild playerindex)
      (bind _ps (CallFunction|GetPSbyIndex playerindex self))
      (Utilities|IsValid _ps
        (:Is%20Valid
          (Default|AddDestroy _ps 1))))))

(fn IsDestroyed
  (return (<= (Variables|Default|Get_heath) 0)))

(fn TakeDamgebyChild
  (params (playerindex :type Integer)))

(fn ProcessDestroybyChild
  (params (playerindex :type Integer)))

(fn ProcessBound
  (Utilities|IsValid self
    (:Is%20Valid
      (if (Ability|HasAuthority)
        (bind _asgs (Utilities|Casting|CastToGS (Game|GetGameState)))
        (if (< (.X (Math|Vector|BreakVector (Transformation|GetActorLocation))) (+ (Variables|/Game/GameState/GS.GS_C|Get_movelength _asgs) (Variables|/Game/GameState/GS.GS_C|Get_startx _asgs)))
          (Actor|DestroyActor))))))